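; First-person player character with gravity-gun style physics interaction, plus standard movement and look input.
; Camera traces find physics objects to push with impulses or grab through a runtime-added PhysicsHandle, which follows SnapPoint each tick until the object is dropped or launched.
; Interact shows the tick-updated reticle billboard while held, then on release traces and messages the hit actor with its component.
; A separate input spawns projectiles from the camera.
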(event EventBeginPlay)

(event EventActorBeginOverlap
  (params (OtherActor :type Actor%20Object%20Reference)))

(event EventTick
  (params (DeltaSeconds :type Float%20%28single-precision%29))
  (Utilities|FlowControl|Sequence
    (:then_0
      (CallFunction|UpdateReticle))
    (:then_1
      (if (Variables|Default|GetIsGunEngaged)
        (CallFunction|UpdatePhysicsHandle)))))

(event Input|ActionEvents|InputActionApplyForce
  (bind _camera (Variables|Default|GetCamera))
  (bind _returnvalue (Transformation|GetWorldLocation _camera))
  (:Pressed
    (bind (_outhit _returnvalue_2) (Collision|LineTraceForObjects _returnvalue (+ (* (Math|Vector|GetForwardVector _camera) 1e+04) _returnvalue) (Utilities|Array|MakeArray (Variables|Default|GetPhysicsObjectType)) false 0 "ForDuration"))
    (if _returnvalue_2
      (bind _output_get (Variables|Default|SetHitPhysicsObject (.HitComponent (Collision|BreakHitResult _outhit)))) ; Because trace only hits physics objects
      (Physics|AddImpulse _output_get (* (Math|Vector|GetForwardVector (Variables|Default|GetCamera)) (Variables|Default|GetImpulseScalar)) "None" (Variables|Default|GetIsVelChange)))))

(event Input|ActionEvents|InputActionInteract
  (bind _camera (Variables|Default|GetCamera))
  (bind _reticlebillboard (Variables|Default|GetReticleBillboard))
  (bind _returnvalue (Transformation|GetWorldLocation _camera))
  (:Pressed
    (Rendering|SetVisibility _reticlebillboard (not (Variables|/Script/Engine.SceneComponent|GetbVisible _reticlebillboard)) false :!label _label))
  (:Released
    (Utilities|FlowControl|Sequence
      (:then_0
        (goto _label))
      (:then_1
        (bind (_outhit _returnvalue_2) (Collision|LineTraceByChannel _returnvalue (+ _returnvalue (* (Math|Vector|GetForwardVector _camera) 1.5e+04)) "TraceTypeQuery1" false 0 "ForDuration"))
        (if _returnvalue_2
          (Class|BPIUseInterface|TraceHitActorwithComponent(Message) (.HitActor (Collision|BreakHitResult _outhit)) (.HitComponent (Collision|BreakHitResult _outhit))))))))

(event Input|ActionEvents|InputActionShootProjectile
  (bind _camera (Variables|Default|GetCamera))
  ;[1 1 1] Shoot Projectile
  (:Pressed
    (Game|SpawnActorfromClass "/Game/Blueprints/MyCustomProjectile.MyCustomProjectile_C" (Math|Transform|MakeTransform (+ (Transformation|GetWorldLocation _camera) (* (Math|Vector|GetForwardVector _camera) 2e+02)) (Transformation|GetWorldRotation _camera)) false 0)))

(event Input|ActionEvents|InputActionShootPickup
  (:Pressed
    (if (Variables|Default|GetIsGunEngaged)
      (CallFunction|DropActor)
      (CallFunction|ShootActor)
      (CallFunction|ResetActorReference))))

(event Input|ActionEvents|InputActionPickup
  (:Pressed
    (if (Variables|Default|GetIsGunEngaged)
      (CallFunction|DropActor)
      (CallFunction|ResetActorReference)
      (else
        (CallFunction|PickUpActor)))))

(event Input|AxisEvents|InputAxisTurn
  (params (AxisValue :type Float%20%28single-precision%29))
  ;[1 1 1] Turn with Mouse
  (Pawn|Input|AddControllerYawInput AxisValue))

(event Input|AxisEvents|InputAxisMoveForward
  (params (AxisValue :type Float%20%28single-precision%29))
  ;[1 1 1] Move Forward/Right
  (Pawn|Input|AddMovementInput (Transformation|GetActorForwardVector) AxisValue false))

(event Input|AxisEvents|InputAxisLookUpRate
  (params (AxisValue :type Float%20%28single-precision%29))
  ;[1 1 1] Lookup with Gamepad
  (Pawn|Input|AddControllerPitchInput (* AxisValue (Utilities|Time|GetWorldDeltaSeconds) (Variables|Default|GetLookUpRateScalar))))

(event Input|AxisEvents|InputAxisLookUp
  (params (AxisValue :type Float%20%28single-precision%29))
  ;[1 1 1] Lookup with Mouse (disabled in VR)
  (Pawn|Input|AddControllerPitchInput AxisValue))

(event Input|AxisEvents|InputAxisMoveRight
  (params (AxisValue :type Float%20%28single-precision%29))
  ;[1 1 1] Move Forward/Right
  (Pawn|Input|AddMovementInput (Transformation|GetActorRightVector) AxisValue false))

(event Input|AxisEvents|InputAxisTurnRate
  (params (AxisValue :type Float%20%28single-precision%29))
  ;[1 1 1] Turn with Keyboard/Gamepad
  (Pawn|Input|AddControllerYawInput (* AxisValue (Utilities|Time|GetWorldDeltaSeconds) (Variables|Default|GetTurnRateScalar))))

(fn ConstructionScript)

(fn UpdateReticle
  (bind (_startpoint _endpoint) (Utilities|ReticlePoints))
  (bind _outhit (Collision|LineTraceByChannel _startpoint _endpoint "TraceTypeQuery1" false 0 "None"))
  (if true
    (LocalVariables|SetReticleLocation (.Location (Collision|BreakHitResult _outhit)))
    (else
      (LocalVariables|SetReticleLocation (.EndPoint (Utilities|ReticlePoints)))))
  (Transformation|SetWorldLocation (Variables|Default|GetReticleBillboard) (LocalVariables|GetReticleLocation) false))

(fn PickUpActor
  (bind _camera (Variables|Default|GetCamera))
  (bind _returnvalue (Transformation|GetWorldLocation _camera))
  (bind (_outhit _returnvalue_2) (Collision|LineTraceForObjects _returnvalue (+ (* (Math|Vector|GetForwardVector _camera) 1e+03) _returnvalue) (Utilities|Array|MakeArray (Variables|Default|GetPhysicsObjectType)) false 0 "ForDuration"))
  (if _returnvalue_2
    (Variables|Default|SetIsGunEngaged true)
    (Variables|Default|SetHitPhysicsObject (.HitComponent (Collision|BreakHitResult _outhit))) ; Because trace only hits physics objects
    (bind _returnvalue_3 (AddComponent|AddPhysicsHandleComponent (Transformation|GetActorTransform)))
    (bind _output_get (Variables|Default|SetPhysicsHandle _returnvalue_3))
    (Class|PhysicsHandleComponent|GrabComponent _output_get (Variables|Default|GetHitPhysicsObject) (.HitBoneName (Collision|BreakHitResult _outhit)) (Transformation|GetWorldLocation (Variables|Default|GetHitPhysicsObject)) (Variables|Default|GetIsConstrainRotation))
    (Collision|SetCollisionResponsetoChannel (Variables|Default|GetHitPhysicsObject) "ECC_Pawn" "ECR_Ignore")
    (Class|PrimitiveComponent|SetAngularDamping (Variables|Default|GetHitPhysicsObject) 1e+01)))

(fn UpdatePhysicsHandle
  (bind _snappoint (Variables|Default|GetSnapPoint))
  (Class|PhysicsHandleComponent|SetTargetLocationandRotation (Variables|Default|GetPhysicsHandle) (Transformation|GetWorldLocation _snappoint) (Transformation|GetWorldRotation _snappoint)))

(fn DropActor
  (bind _hitphysicsobject (Variables|Default|GetHitPhysicsObject))
  (Variables|Default|SetIsGunEngaged false)
  (Physics|Components|PhysicsHandle|ReleaseComponent (Variables|Default|GetPhysicsHandle))
  (Collision|SetCollisionResponsetoChannel _hitphysicsobject "ECC_Pawn" "ECR_Block")
  (Class|PrimitiveComponent|WakeRigidBody _hitphysicsobject "None"))

(fn ResetActorReference
  (Variables|Default|SetHitPhysicsObject 0))

(fn ShootActor
  (Physics|AddImpulse (Variables|Default|GetHitPhysicsObject) (* (Math|Vector|GetForwardVector (Variables|Default|GetCamera)) (Variables|Default|GetImpulseScalar)) "None" (Variables|Default|GetIsVelChange)))