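; BP_Celestial is a celestial body actor that orbits a ParentActor.
; BeginPlay creates a dynamic material instance on slot 0 from MaterialInstance, if one is set.
; Tick passes through a short Delay that throttles updates, then rotates the body's offset from ParentActor in pitch by Rotation and adds it to the parent's current location.
; The orbit steps by a fixed angle per update, without delta-time scaling.
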(event EventBeginPlay
  (bind _material_instance (Variables|Default|GetMaterial%20Instance))
  (Utilities|IsValid _material_instance
    (:Is%20Valid
      (Rendering|Material|CreateDynamicMaterialInstance 0 _material_instance :!class /Script/Engine.PrimitiveComponent))))

(event EventActorBeginOverlap
  (params (OtherActor :type Actor%20Object%20Reference)))

(event EventTick
  (params (DeltaSeconds :type Float%20%28single-precision%29))
  (bind _self self)
  (bind _parent_actor (Variables|Default|GetParent%20Actor))
  (bind _returnvalue (Transformation|GetActorLocation _parent_actor))
  (Utilities|FlowControl|Delay 0.02)
  (Utilities|IsValid (Variables|Default|GetParent%20Actor)
    (:Is%20Valid
      (Transformation|SetActorLocation _self (+ _returnvalue (Math|Vector|RotateVector (- (Transformation|GetActorLocation _self) _returnvalue) (Math|Rotator|MakeRotator (Variables|Default|GetRotation) 0.0 0.0))) false))))

(fn ConstructionScript)