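; BP_MeshSpline is a construction-script tool that places copies of a chosen static mesh along a spline.
; It divides the spline length by LengthInterval and adds a mesh component at each step, matching the spline's world location and rotation without deforming the mesh.
; Each component gets MaterialInstance on its first material slot; the event graph has no runtime logic.
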(event EventBeginPlay)

(event EventActorBeginOverlap
  (params (OtherActor :type Actor%20Object%20Reference)))

(event EventTick
  (params (DeltaSeconds :type Float%20%28single-precision%29)))

(fn ConstructionScript
  (bind _spline (Variables|Default|GetSpline))
  (Utilities|IsValid (Variables|Default|GetMesh%20To%20Spawn)
    (:Is%20Valid
      (bind _output_get (Variables|Default|SetTot%20Length (Spline|GetSplineLength)))
      (bind _output_get_2 (Variables|Default|SetNumber%20Intervals (Math|Float|Floor (/ _output_get (Variables|Default|GetLength%20Interval)))))
      (for _index (range 0 _output_get_2)
        (bind _returnvalue (AddComponent|AddStaticMeshComponent false))
        (Components|StaticMesh|SetStaticMesh _returnvalue (Variables|Default|GetMesh%20To%20Spawn))
        (Class|SceneComponent|Attachto _returnvalue (Variables|Default|GetScene) "None" "KeepRelativeOffset" true)
        (Transformation|SetWorldLocationAndRotation _returnvalue (Class|SplineComponent|GetWorldLocationatDistanceAlongSpline _spline (* _index (Variables|Default|GetLength%20Interval))) (Class|SplineComponent|GetWorldRotationatDistanceAlongSpline _spline (* _index (Variables|Default|GetLength%20Interval))) false)
        (Rendering|Material|SetMaterial _returnvalue 0 (Variables|Default|GetMaterial%20Instance))))))