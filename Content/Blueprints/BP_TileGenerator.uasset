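; BP_TileGenerator is a construction-time tile generator that scales a Cube and can lay out an X by Y grid of static mesh components attached to it.
; Each added tile is offset by Space, with random height and rotation variation, and the Cube is turned toward EndPoint.
; EndPoint is zeroed just before its non-zero X check, so as written the grid branch never runs.
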(event EventBeginPlay)

(event EventActorBeginOverlap
  (params (OtherActor :type Actor%20Object%20Reference)))

(event EventTick
  (params (DeltaSeconds :type Float%20%28single-precision%29)))

(fn ConstructionScript
  (bind _returnvalue (Transformation|GetActorLocation))
  (bind _scale (Variables|Default|GetScale))
  (bind _height_variation (Variables|Default|GetHeight%20Variation))
  (bind _space (Variables|Default|GetSpace))
  (bind _rotation_variation (Variables|Default|GetRotation%20Variation))
  (bind _returnvalue_2 (/ _rotation_variation 2.0))
  (bind _returnvalue_3 (/ _height_variation 2.0))
  (bind _returnvalue_4 (* _returnvalue_2 -1.0))
  (bind _returnvalue_5 (Math|Random|RandomFloatinRange _returnvalue_4 _returnvalue_2))
  (Transformation|SetWorldScale3D (Variables|Default|GetCube) (Math|Vector|MakeVector _scale _scale _scale))
  (bind _output_get (LocalVariables|SetEnd%20Point (Math|Vector|MakeVector 0.0 0.0 0.0)))
  (if (Math|Vector|NotEqual(Vector) (* _output_get "1.000000, 0, 0") "0, 0, 0" 0.0)
    (for _index (range 0 (Variables|Default|GetX))
      (for _index_2 (range 0 (Variables|Default|GetY))
        (if (!= (+ _index _index_2) 0)
          (bind _returnvalue_6 (AddComponent|AddStaticMeshComponent false))
          (Class|SceneComponent|Attachto _returnvalue_6 (Variables|Default|GetCube) "None" "KeepRelativeOffset" true)
          (Transformation|SetRelativeLocation _returnvalue_6 (Math|Vector|MakeVector (* _index _space) (* _index_2 _space) (Math|Random|RandomFloatinRange (* _returnvalue_3 -1.0) _returnvalue_3)) false)
          (Transformation|SetRelativeRotation _returnvalue_6 (Math|Rotator|MakeRotator _returnvalue_5 _returnvalue_5 _returnvalue_5) false)
          (Transformation|SetRelativeRotation (Variables|Default|GetCube) (Math|Rotator|FindLookatRotation _returnvalue (+ (LocalVariables|GetEnd%20Point) _returnvalue)) false))))))