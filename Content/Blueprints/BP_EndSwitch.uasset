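; BP_EndSwitch is a look-trace switch that nudges a referenced ActorToMove, and itself, along each actor's local X axis.
; A hit on DownCube moves both by negative MoveSpeed, while any other component moves them by positive MoveSpeed.
; Every hit also restarts a timeline driving LerpAlpha on DownCube's dynamic M_Tube material, created in the Construction Script.
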(event EventBeginPlay)

(event EventActorBeginOverlap
  (params (OtherActor :type Actor%20Object%20Reference)))

(event EventTick
  (params (DeltaSeconds :type Float%20%28single-precision%29)))

(event EventTraceLookHitActorwithComponent
  (params (Component :type Primitive%20Component%20Object%20Reference))
  (bind _movespeed (Variables|Default|GetMoveSpeed))
  (if (== Component (Variables|Default|GetDownCube))
    (Variables|Default|SetThisMoveSpeed (* _movespeed -1.0))
    (else
      (Variables|Default|SetThisMoveSpeed _movespeed)))
  (Transformation|AddActorLocalOffset (Variables|Default|GetActorToMove) (Math|Vector|MakeVector (Variables|Default|GetThisMoveSpeed) 0.0 0.0) false)
  (Transformation|AddActorLocalOffset self (Math|Vector|MakeVector (Variables|Default|GetThisMoveSpeed) 0.0 0.0) false)
  (bind _alpha1 (Timeline|Timeline_0 PlayFromStart)
    (:Update
      (Rendering|Material|SetScalarParameterValue (Variables|Default|GetDownDynamicMaterial) "LerpAlpha" _alpha1 :!class /Script/Engine.MaterialInstanceDynamic))))

(fn ConstructionScript
  (bind _returnvalue (Rendering|Material|CreateDynamicMaterialInstance (Variables|Default|GetDownCube) 0 "/Game/MyMaterials/M_Tube.M_Tube" :!class /Script/Engine.PrimitiveComponent))
  (Variables|Default|SetDownDynamicMaterial _returnvalue))